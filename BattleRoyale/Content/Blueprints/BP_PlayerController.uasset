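; BP_PlayerController is the player controller that manages the lobby, in-game and map widgets, plus spectating after a kill.
; The local controller shows the lobby on BeginPlay, then GameBegunEvent swaps it for the player screen and prints the net role.
; Holding the Map input shows a lazily created, cached map widget.
; BeginTheSpectating possesses a spectator pawn attached to the killer; its spectator and post-match screen events are empty stubs.
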(event Custom|Show%20In%20Game%20HUD
  ;[0.2422 1 0] PlayerScreen From C++
  (if (Pawn|IsLocalController)
    (bind _returnvalue (UserInterface|CreateWidget "/Game/UI/WBP_PlayerScreen.WBP_PlayerScreen_C" self))
    (bind _output_get (Variables|Default|SetInGameHUD _returnvalue))
    (UserInterface|Viewport|AddtoViewport _output_get 0)))

(event Custom|BeginTheSpectating
  (params (Killer :type Player%20Pawn%20Object%20Reference))
  ;[1 0.008127 0] Spec Setup
  (Utilities|IsValid Killer
    (:Is%20Valid
      (Variables|Default|SetKillledBy Killer)
      (bind _returnvalue (Game|SpawnActorfromClass "/Game/Blueprints/BP_SpectatorPawn.BP_SpectatorPawn_C" (Transformation|GetActorTransform) "Undefined" self 0))
      (Transformation|AttachActorToActor _returnvalue (Variables|Default|GetKillledBy) "None" "SnapToTarget" "SnapToTarget" "SnapToTarget" true)
      (Pawn|Possess _returnvalue)
      (CallFunction|AddSpectatorScreen))
    (:Is%20Not%20Valid
      (CallFunction|AddPostMatchScreen))))

(event Custom|Add%20Post%20Match%20Screen
  ;[1 0.008127 0] Spec Setup
)

(event Custom|Add%20Spectator%20Screen
  ;[1 0.008127 0] Spec Setup
)

(event EventBeginPlay
  ;[0.1192 1 0] Create Lobby Widget From C++
  (if (Pawn|IsLocalController)
    (bind _returnvalue (UserInterface|CreateWidget "/Game/UI/WBP_Lobby.WBP_Lobby_C" self))
    (bind _output_get (Variables|Default|SetLobbyHUD _returnvalue))
    (UserInterface|Viewport|AddtoViewport _output_get 0)))

(event EventTick
  (params (DeltaSeconds :type Float%20%28single-precision%29)))

(event EventGameBegunEvent
  (bind _lobbyhud (Variables|Default|GetLobbyHUD))
  ;[0.4055 1 0] After Game Begun From C++
  (Utilities|IsValid _lobbyhud
    (:Is%20Valid
      (Widget|RemovefromParent _lobbyhud)
      (CallFunction|ShowinGameHUD)
      (Development|PrintString (Utilities|String|EnumtoString (Networking|GetLocalRole)) true true "(R=0.000000,G=0.660000,B=1.000000,A=1.000000)" 1e+01))))

(event Input|ActionEvents|InputActionMap
  (params (Key :type Key%20Structure :default "None"))
  (:Pressed
    (Utilities|IsValid (Variables|Default|GetMapHUD)
      (:Is%20Valid
        _)
      (:Is%20Not%20Valid
        (bind _returnvalue (UserInterface|CreateWidget "/Game/UI/WBP_MainMap.WBP_MainMap_C" self))
        (Variables|Default|SetMapHUD _returnvalue)))
    (UserInterface|Viewport|AddtoViewport (Variables|Default|GetMapHUD) 0))
  (:Released
    (Widget|RemovefromParent (Variables|Default|GetMapHUD))))

(fn ConstructionScript)