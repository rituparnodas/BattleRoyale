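; Base gun Blueprint that manages clip and spare ammo, with firing and ammo pickups processed only on the server.
; OnFired decrements the clip and calls Reload when empty, while GiveAmmo tops up the clip and stores overflow up to the spare cap.
; ReloadBP flags the owning pawn as reloading during a fixed delay, then refills from spare ammo.
; HasAmmo reports a non-empty clip; the ammo and owner setup is disconnected from BeginPlay.
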(event Custom|Give%20Ammo
  (params (Ammo%20To%20Give :type Integer))
  ;[1 0.7784 0] Give Ammo To Weapon
  (Networking|SwitchHasAuthority
    (:Authority
      (Variables|Default|SetCurrentAmmoBP (+ (Math|Integer|Min(Integer) Ammo%20To%20Give (- (Variables|Default|GetClipSize_0) (Variables|Default|GetCurrentAmmoBP))) (Variables|Default|GetCurrentAmmoBP)))
      (if (> (- Ammo%20To%20Give (Math|Integer|Min(Integer) Ammo%20To%20Give (- (Variables|Default|GetClipSize_0) (Variables|Default|GetCurrentAmmoBP)))) 0)
        (Variables|Default|SetCurrentSpareAmmoBP (+ (Variables|Default|GetCurrentSpareAmmoBP) (Math|Integer|Min(Integer) (- Ammo%20To%20Give (Math|Integer|Min(Integer) Ammo%20To%20Give (- (Variables|Default|GetClipSize_0) (Variables|Default|GetCurrentAmmoBP)))) (- (Variables|Default|GetMaxSpareAmmoBP) (Variables|Default|GetCurrentSpareAmmoBP)))))))))

(event Custom|On%20Fired
  (bind _currentammobp (Variables|Default|GetCurrentAmmoBP))
  ;[1 0.8915 0] When Fire Gun
  (Networking|SwitchHasAuthority
    (:Authority
      (Math|Integer|DecrementInt _currentammobp
        (:%20%20
          (if (<= _currentammobp 0)
            (CallFunction|Reload)))))))

(event Custom|ReloadBP
  (bind _currentowner_0 (Variables|Default|GetCurrentOwner_0))
  ;[1 0.8727 0] Reload
  (Variables|/Game/Blueprints/PlayerPawn.PlayerPawn_C|SetReloading? _currentowner_0 true)
  (Utilities|FlowControl|Delay 2.0)
  (Variables|Default|SetCurrentAmmoBP (Math|Integer|Min(Integer) (Variables|Default|GetCurrentSpareAmmoBP) (Variables|Default|GetClipSize_0)))
  (Variables|Default|SetCurrentSpareAmmoBP (Math|Integer|Max(Integer) (- (Variables|Default|GetCurrentSpareAmmoBP) (Math|Integer|Min(Integer) (Variables|Default|GetCurrentSpareAmmoBP) (Variables|Default|GetClipSize_0)))))
  (Variables|/Game/Blueprints/PlayerPawn.PlayerPawn_C|SetReloading? _currentowner_0 false))

(event EventBeginPlay
  ;[1 0.8096 0] Setup Ammo
)

(fn ConstructionScript)

(fn HasAmmo?
  (return (> (Variables|Default|GetCurrentAmmoBP) 0)))