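; Player character for a networked shooter with a safe zone and flight, layering Blueprint logic over C++-driven movement, reload and health.
; Flight retunes CharacterMovement until a grounded hit, a looping timer toggles post-process outside the zone, and zero Health drops the gun as a server-spawned pickup.
; RepNotifies attach weapons, play reload montages and ragdoll the body.
; An older Blueprint weapon and health path remains, partly disconnected.
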(event OnComponentHit(CapsuleComponent)
  (params (HitComponent :type Primitive%20Component%20Object%20Reference) (OtherActor :type Actor%20Object%20Reference) (OtherComp :type Primitive%20Component%20Object%20Reference) (NormalImpulse :type Vector :default "0, 0, 0") (Hit :type Hit%20Result%20Structure%20%28by%20ref%29))
  ;[0.1988 1 0] Update Movement From C++
  (if (AI|Components|NavMovement|IsMovingonGround (Variables|Character|GetCharacterMovement))
    (Class|BattleRoyaleCharacter|SetFlying false)))

(event Custom|Give%20The%20Weapon
  (params (Weapon :type Gun%20Base%20Class%20Reference))
  (bind _self self)
  ;[1 0 0.02677] Spawn Weapon
  (bind _returnvalue (Game|SpawnActorfromClass Weapon (Transformation|GetActorTransform) "AlwaysSpawn" _self 0 0 _self))
  (Variables|DefaultWeapon|SetWeapon _returnvalue))

(event Custom|Server%20Fire%20Gun
  (bind _returnvalue (Pawn|GetController))
  (bind _self self)
  (bind _mesh1p (Variables|Default|GetMesh1P))
  (bind _returnvalue_2 (Transformation|GetWorldTransform _mesh1p))
  (bind (_outlocation _outrotation) (Actor|GetActorEyesViewPoint _returnvalue))
  ;[1 0.01151 0.1412] Server fire Logic
  (Default|OnFired (Variables|DefaultWeapon|GetWeapon_2))
  (bind _outhit (Collision|LineTraceByChannel _outlocation (+ _outlocation (* (Math|Rotator|GetRotationXVector _outrotation) 10000)) "TraceTypeQuery1" false (Utilities|Array|MakeArray self) "ForDuration"))
  (bind _asplayer_pawn (Utilities|Casting|CastToPlayerPawn (.HitActor (Collision|BreakHitResult _outhit)))
    (:then
      (Game|Damage|ApplyDamage _asplayer_pawn (Variables|/Script/BattleRoyale.GunBase|GetDamage (Variables|DefaultWeapon|GetWeapon)) (Pawn|GetController _self) _self "/Script/Engine.DamageType")
      (Effects|SpawnEmitteratLocation "/Game/M5VFXVOL2/Particles/Fire/Fire_00.Fire_00" (.location _returnvalue_2) (.rotation _returnvalue_2) (.scale _returnvalue_2)))
    (:CastFailed
      (Development|PrintString "failed"))))

(event Custom|FireGun
  ;[1 0 0.1797] Client Side Shooting
)

(event Custom|Modify%20Health
  (params (Health :type Float%20%28single-precision%29))
  ;[1 0 0.1826] Modify Health
  (Networking|SwitchHasAuthority
    (:Authority
      (Variables|Health|SetBPHealth (Math|Float|Clamp(Float) (- (Variables|Health|GetBPHealth) Health) 0.0 (Variables|Health|GetMaxHealth_0))))))

(event Custom|KillByPlayer
  (params (Killer :type Player%20Pawn%20Object%20Reference))
  ;[1 0 0.1085] TakeDamage
  (Variables|Default|SetKilled%20By%20BP Killer))

(event Custom|killed%20By%20Environment
  (params (Killer :type Actor%20Object%20Reference)))

(event Custom|Play%20Reload%20Animaion
  (params (Is%20Local%20Player%20? :type Boolean))
  ;[1 0 0.03483] Animation reload
  (if Is%20Local%20Player%20?
    (Animation|Montage|PlayMontage (Variables|Default|GetMesh1P) "/Game/AnimStarterPack/Reload_FPS_Montage1.Reload_FPS_Montage1")
    (else
      (Animation|Montage|PlayMontage (Variables|Character|GetMesh) "/Game/AnimStarterPack/Reload_Montage.Reload_Montage"))))

(event Custom|MulticastFireFX
  (bind _gun (Variables|Default|GetGun))
  (bind _thirdpersongun (Variables|/Script/BattleRoyale.GunBase|GetThirdPersonGun _gun))
  (bind _returnvalue (Transformation|GetSocketTransform _thirdpersongun "Muzzle" "RTS_World"))
  (Utilities|IsValid _gun
    (:Is%20Valid
      (Effects|SpawnEmitteratLocation "/Game/M5VFXVOL2/Particles/Reference/Fireloop/2_bonefirethin_pt.2_bonefirethin_pt" (.location _returnvalue) (.rotation _returnvalue) (.scale _returnvalue)))))

(event Custom|Drop%20Current%20Weapon
  (bind _gun (Variables|Default|GetGun))
  ;[1 0 0.02557] Drop pickup
  (Networking|SwitchHasAuthority
    (:Authority
      (Game|SpawnActorfromClass (Variables|/Script/BattleRoyale.GunBase|GetWeaponPickup _gun) (Class|BattleRoyaleCharacter|GetPickupSpawnTransform) "Undefined" 0 (Variables|/Script/BattleRoyale.GunBase|GetCurrentAmmo _gun) (Variables|/Script/BattleRoyale.GunBase|GetCurrentBagAmmo _gun) true 0))))

(event EventBeginPlay
  (Utilities|Time|SetTimerbyFunctionName self "ChangeColor" 0.15 true))

(event Collision|EventActorBeginOverlap
  (params (OtherActor :type Actor%20Object%20Reference)))

(event EventTick
  (params (DeltaSeconds :type Float%20%28single-precision%29))
  ;[0.286 1 0] From C++
  (if (and (<= (Variables|Default|GetHealth) 0.0) (not (Variables|Default|GetDead?)))
    (Variables|Default|SetDead? true)
    (Class|BattleRoyaleCharacter|DropCurrentWeapon)))

(event Game|Damage|EventAnyDamage
  (params (Damage :type Float%20%28single-precision%29) (DamageType :type Damage%20Type%20Object%20Reference) (InstigatedBy :type Controller%20Object%20Reference) (DamageCauser :type Actor%20Object%20Reference))
  ;[1 0 0.1085] TakeDamage
)

(event EventOnGunReload
  (params (IsLocalPlayer :type Boolean))
  ;[0.2637 1 0] Reload From C++
  (Variables|Default|SetReloadAnim true)
  (Utilities|FlowControl|Delay 2.0)
  (Variables|Default|SetReloadAnim false))

(event EventUpdateMovement
  (bind _charactermovement (Variables|Character|GetCharacterMovement))
  (bind _bflying (Variables|Default|GetbFlying))
  ;[0.1988 1 0] Update Movement From C++
  (Variables|/Script/Engine.CharacterMovementComponent|SetMaxWalkSpeed _charactermovement (select _bflying 2e+03 6e+02))
  (Variables|/Script/Engine.CharacterMovementComponent|SetAirControl _charactermovement (select _bflying 1.0 0.05))
  (Variables|/Script/Engine.CharacterMovementComponent|SetGravityScale _charactermovement (select _bflying 0.2 1.0))
  (Variables|/Script/Engine.CharacterMovementComponent|SetMaxAcceleration _charactermovement (select _bflying 512.0 2048.0)))

(event Input|ActionEvents|InputActionFire
  (params (Key :type Key%20Structure :default "None"))
  ;[1 0.01151 0.1412] Server fire Logic
)

(fn ConstructionScript)

(fn OnRepWeapon
  (bind _weapon (Variables|DefaultWeapon|GetWeapon))
  (Transformation|AttachComponentToComponent (Variables|/Script/BattleRoyale.GunBase|GetThirdPersonGun _weapon) (Variables|Character|GetMesh) "WeaponSocket" "SnapToTarget" "SnapToTarget" "SnapToTarget" true)
  (Transformation|AttachComponentToComponent (Variables|/Script/BattleRoyale.GunBase|GetFirstPersonGun _weapon) (Variables|Default|GetMesh1P) "WeaponSocket" "SnapToTarget" "SnapToTarget" "SnapToTarget" true))

(fn OnRepKilledBYBP
  (bind _mesh (Variables|Character|GetMesh))
  (Collision|SetCollisionEnabled _mesh "PhysicsOnly")
  (Physics|SetSimulatePhysics _mesh true)
  (Collision|SetCollisionEnabled (Variables|Default|GetCapsuleComponent) "NoCollision")
  (Components|Movement|StopMovementImmediately (Variables|Character|GetCharacterMovement)))

(fn OnRepBPHealth)

(fn OnRepReloading?
  (if (Variables|Default|GetReloading?)
    (CallFunction|PlayReloadAnimaion (Pawn|IsLocallyControlled))))

(fn OnRepCurrentGunPickup)

(fn ChangeColor
  (bind _postprocess (Variables|Default|GetPostProcess))
  (bind _asbp_game_state (Utilities|Casting|CastToBP_GameState (Game|GetGameState)))
  (Utilities|IsValid (Variables|/Script/BattleRoyale.BRGameStateBase|GetSafeZone _asbp_game_state)
    (:Is%20Valid
      (if (Variables|/Script/BattleRoyale.BRSafeZone|GetbOutsideZone (Variables|/Script/BattleRoyale.BRGameStateBase|GetSafeZone _asbp_game_state))
        (Variables|/Script/Engine.PostProcessComponent|SetbEnabled _postprocess true)
        (else
          (Variables|/Script/Engine.PostProcessComponent|SetbEnabled _postprocess false))))))